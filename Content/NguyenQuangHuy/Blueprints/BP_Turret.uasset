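; BP_Turret is an enemy turret that detects a Player-tagged pawn through PawnSensing and locks onto it.
; One looping timer turns it in yaw toward the target, and another fires BP_CannonBall from BulletSpawn at a fixed interval.
; Firing stops when the target reports it is dead or becomes invalid, while tracking stops and releases the lock only when the target is invalid.
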(event `self.PawnSensing.OnSeePawn`
  (params (Pawn :type "Pawn Object Reference"))
  ;[1 1 1] Event see target
  (if (`self.ActorHasTag` Pawn "Player")
    (`/Engine/EditorBlueprintResources/StandardMacros.IsValid` Pawn
      (:`Is Valid`
        (if (not (`self.HasTarget?`))
          (set `self.HasTarget?` true)
          (set `self.TargetPawn` Pawn)
          (`self.TrackTarget`)
          (`self.Fire Loop`))))))

(event `TrackTarget`
  ;[1 1 1] Rotate Turret to face target
  (bind _returnvalue (`KismetSystemLibrary.K2_SetTimerDelegate` (delegate `MoveTurret`) 0.001 true))
  (set `self.TimerRef` _returnvalue))

(event `MoveTurret`
  (bind _targetpawn (`self.TargetPawn`))
  (bind (_returnvalue_roll _returnvalue_pitch _returnvalue_yaw) (`KismetMathLibrary.BreakRotator` (`KismetMathLibrary.RInterpTo` (`self.K2_GetActorRotation`) (`KismetMathLibrary.FindLookAtRotation` (`self.K2_GetActorLocation`) (`self.K2_GetActorLocation` _targetpawn)) (`GameplayStatics.GetWorldDeltaSeconds`) 100.0)))
  ;[1 1 1] Rotate Turret to face target
  (`/Engine/EditorBlueprintResources/StandardMacros.IsValid` _targetpawn
    (:`Is Valid`
      (`self.K2_SetActorRotation` (`KismetMathLibrary.MakeRotator` 0.0 0.0 _returnvalue_yaw)))
    (:`Is Not Valid`
      (`KismetSystemLibrary.K2_ClearAndInvalidateTimerHandle` (`self.TimerRef`))
      (set `self.HasTarget?` false))))

(event `Fire Loop`
  ;[1 1 1] Fire Loop Logic
  (bind _returnvalue (`KismetSystemLibrary.K2_SetTimerDelegate` (delegate `FireCannon`) 0.5 true))
  (set `self.FireTimerRef` _returnvalue))

(event `FireCannon`
  ;[1 1 1] Fire Loop Logic
  (if (`self.HasTarget?`)
    (bind _targetpawn (`self.TargetPawn`)
      (:`then`
        (bind _isdead_ (message `/Game/NguyenQuangHuy/InterFaces/BPI_PlayerCharacter.GetIsPlayerDead?` _targetpawn))
        (if _isdead_
          (`KismetSystemLibrary.K2_ClearAndInvalidateTimerHandle` (`self.FireTimerRef`))
          (else
            (`|SpawnActorFromClass` "/Game/NguyenQuangHuy/Blueprints/BP_CannonBall.BP_CannonBall_C" (`SceneComponent.K2_GetComponentToWorld` (`self.BulletSpawn`)) "Undefined" "MultiplyWithRoot" null null))))
      (:`else`
        (`KismetSystemLibrary.K2_ClearAndInvalidateTimerHandle` (`self.FireTimerRef`) :!label _label)))
    (else
      (goto _label))))

(fn `UserConstructionScript`)