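; BP_BlockDamageable is a destructible block actor that breaks apart once it takes enough damage.
; It resets Life to LifeMax on BeginPlay and subtracts incoming AnyDamage while Life is above zero.
; When Life reaches zero, a DoOnce calls Explode, which spawns the P_Brick particle at the FX component's location and destroys the actor.
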(event `self.ReceiveBeginPlay`
  (set `self.Life` (`self.LifeMax`)))

(event `self.ReceiveAnyDamage`
  (params (Damage :type "Float (single-precision)") (DamageType :type "DamageType Object Reference") (InstigatedBy :type "Controller Object Reference") (DamageCauser :type "Actor Object Reference"))
  (if (> (`self.Life`) 0.0)
    (bind _output_get (set `self.Life` (- (`self.Life`) Damage)))
    (if (<= _output_get 0.0)
      (`/Engine/EditorBlueprintResources/StandardMacros.DoOnce` false
        (:`Completed`
          (`self.Explode`))))))

(event `Explode`
  (`GameplayStatics.SpawnEmitterAtLocation` "/Game/Realistic_Starter_VFX_Pack_Vol2/Particles/Hit/P_Brick.P_Brick" (`SceneComponent.K2_GetComponentLocation` (`self.FX`)))
  (`self.K2_DestroyActor`))

(fn `UserConstructionScript`)