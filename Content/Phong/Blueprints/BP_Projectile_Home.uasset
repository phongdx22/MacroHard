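; BP_Projectile_Home is a projectile that picks a player tank as its homing target.
; When OverlapSphere begins overlapping a BP_TankPlayer that has no valid PowerUpsComponents component, it sets that tank's TankBody as the ProjectileMovement homing target.
; A DoOnce locks the projectile onto the first qualifying tank, so later overlaps do not retarget it.
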(event `self.OverlapSphere.OnComponentBeginOverlap`
  (params (OverlappedComponent :type "PrimitiveComponent Object Reference") (OtherActor :type "Actor Object Reference") (OtherComp :type "PrimitiveComponent Object Reference") (OtherBodyIndex :type Integer) (bFromSweep :type Boolean) (SweepResult :type "HitResult Structure (by ref)"))
  (bind _asbp_tank_player (cast `/Game/Phong/Blueprints/BP_TankPlayer` OtherActor))
  (`/Engine/EditorBlueprintResources/StandardMacros.IsValid` (`self.GetComponentByClass` _asbp_tank_player "/Game/HAN23080480/Objects/PowerUpsComponents.PowerUpsComponents_C")
    (:`Is Not Valid`
      (`/Engine/EditorBlueprintResources/StandardMacros.DoOnce` false
        (:`Completed`
          (set `ProjectileMovementComponent.HomingTargetComponent` (`/Game/Phong/Blueprints/BP_TankPlayer.TankBody` _asbp_tank_player) (`self.ProjectileMovement`)))))))

(fn `UserConstructionScript`
  (`parent.UserConstructionScript`))