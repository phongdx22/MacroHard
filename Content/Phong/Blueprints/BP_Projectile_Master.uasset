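; Master Blueprint for a ricocheting projectile that damages actors tagged Tank on overlap and is then destroyed.
; On other overlaps, a forward line trace finds the surface, and the bullet mirrors its rotation and velocity about the hit normal.
; A DoOnce gates each bounce; at the bounce limit it plays a wall-hit sound and destroys itself.
; When destroyed, it tells its instigator to update the bullet count message.
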(event `self.ReceiveActorBeginOverlap`
  (params (OtherActor :type "Actor Object Reference"))
  ;[1 1 1] Bullet bounce
  (if (`self.ActorHasTag` OtherActor "Tank")
    (`GameplayStatics.ApplyDamage` OtherActor (`self.Base Damage`))
    (`self.K2_DestroyActor`)
    (else
      (bind (_outhit _returnvalue _origin _forward) (`self.TestTraceDetectionEnvironment`))
      (`/Engine/EditorBlueprintResources/StandardMacros.DoOnce` false :!label _label
        (:`Completed`
          (bind _canbounce_ (`self.CheckIfCanBounce`))
          (if _canbounce_
            (`/Engine/EditorBlueprintResources/StandardMacros.IncrementInt` (`self.BounceCount`)
              (:`  `
                (`self.Bounce` _outhit _origin _forward)
                (goto _label :!via `Reset`)))
            (else
              (`GameplayStatics.SpawnSoundAtLocation` "/Game/NguyenQuangHuy/Assets/SFX/SFX/S_BulletHitWall.S_BulletHitWall" (`SceneComponent.K2_GetComponentLocation` (`self.ForwardArrow`)) (struct) 1.0 1.0 0.0 null null)
              (`self.K2_DestroyActor`))))))))

(event `self.ReceiveDestroyed`
  (bind _instigator_ref (`self.Instigator REF`))
  ;[1 1 1] Bullet bounce
  (`/Engine/EditorBlueprintResources/StandardMacros.IsValid` _instigator_ref
    (:`Is Valid`
      (message `/Game/NguyenQuangHuy/InterFaces/BPI_BulletCount.UpdateBulletCount` _instigator_ref))))

(fn `Bounce`
  (params (Hit :type "HitResult Structure") (Origin :type "Vector Structure") (Forward :type "Vector Structure"))
  (bind (_bblockinghit _binitialoverlap _time _distance _location _impactpoint _normal _impactnormal) (`GameplayStatics.BreakHitResult` Hit))
  (`self.K2_SetActorRotation` (`KismetMathLibrary.FindLookAtRotation` (+ _impactpoint _normal) (+ _impactpoint (`KismetMathLibrary.MirrorVectorByNormal` (- Forward Origin) _normal))))
  (set `MovementComponent.Velocity` (`KismetMathLibrary.MirrorVectorByNormal` (`MovementComponent.Velocity` (`self.ProjectileMovement`)) _impactnormal) (`self.ProjectileMovement`))
  (`GameplayStatics.SpawnSoundAtLocation` "/Game/NguyenQuangHuy/Assets/SFX/SFX/S_Ricochet.S_Ricochet" (`SceneComponent.K2_GetComponentLocation` (`self.ForwardArrow`)) (struct) 1.0 1.0 0.0 null null))

(fn `CheckIfCanBounce`
  (returns (`CanBounce?` :type Boolean))
  (if (< (`self.BounceCount`) (`self.BounceCountMax`))
    (return true)
    (else
      (return false))))

(fn `TestTraceDetectionDamageable`
  (returns (OutHit :type "HitResult Structure") (ReturnValue :type Boolean) (Origin :type "Vector Structure") (Forward :type "Vector Structure"))
  (bind _forwardarrow (`self.ForwardArrow`))
  (bind _returnvalue (`SceneComponent.K2_GetComponentLocation` _forwardarrow))
  (`/Engine/EditorBlueprintResources/StandardMacros.IsValid` _forwardarrow
    (:`Is Valid`
      (bind (_outhit _returnvalue_2) (`KismetSystemLibrary.LineTraceSingle` _returnvalue (+ _returnvalue (* (`SceneComponent.GetForwardVector` _forwardarrow) (`self.TraceDistance`))) "TraceTypeQuery5"))
      (return _outhit _returnvalue_2 (0.0 0.0 0.0) (0.0 0.0 0.0)))))

(fn `TestTraceDetectionEnvironment`
  (returns (OutHit :type "HitResult Structure") (ReturnValue :type Boolean) (Origin :type "Vector Structure") (Forward :type "Vector Structure"))
  (bind _forwardarrow (`self.ForwardArrow`))
  (bind _returnvalue (`SceneComponent.K2_GetComponentLocation` _forwardarrow))
  (bind _returnvalue_2 (+ _returnvalue (* (`SceneComponent.GetForwardVector` _forwardarrow) (`self.TraceDistance`))))
  (bind (_outhit _returnvalue_3) (`KismetSystemLibrary.LineTraceSingle` _returnvalue _returnvalue_2 "TraceTypeQuery4"))
  (return _outhit _returnvalue_3 _returnvalue _returnvalue_2))

(fn `UserConstructionScript`)