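; BP_PlayerTank_Blue is the blue-team variant of a parent player tank Blueprint.
; On BeginPlay it runs the parent logic, then sets the health bar widget's colour to blue.
; It also records its starting transform as the spawn transform and sets TankColour to "Blue"; both steps run only if the health bar cast succeeds.
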(event `self.ReceiveBeginPlay`
  (`parent.ReceiveBeginPlay`)
  (bind _aswbp_health_bar (cast `/Game/HAN23080480/UI/IngameHUD/WBP_HealthBar` (`WidgetComponent.GetUserWidgetObject` (`self.Widget_HealthBar`))))
  (set `/Game/HAN23080480/UI/IngameHUD/WBP_HealthBar.HealthBarColour` (struct :`R` 0.02 :`G` 0.14 :`B` 0.58 :`A` 1.0) _aswbp_health_bar)
  (set `self.SpawnTransform` (`self.GetTransform`))
  (set `self.TankColour` "Blue"))

(fn `UserConstructionScript`
  (`parent.UserConstructionScript`))