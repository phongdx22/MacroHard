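; BP_ModePicker_Fiesta is the mode picker object for Fiesta Mode, described as Classic Mode with power-up pickups.
; On BeginPlay it casts its Widget component's widget to WBP_ModeDescription and fills in the title and two description lines.
; It then sets LevelName to the Fiesta level, only if that cast succeeds.
; The construction script only calls its parent, and no logic here uses LevelName.
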(event `self.ReceiveBeginPlay`
  (bind _aswbp_mode_description (cast `/Game/HAN23080480/UI/IngameHUD/WBP_ModeDescription` (`WidgetComponent.GetWidget` (`self.Widget`))))
  (`TextBlock.SetText` (`/Game/HAN23080480/UI/IngameHUD/WBP_ModeDescription.TextBlock_Title` _aswbp_mode_description) "Fiesta Mode")
  (`TextBlock.SetText` (`/Game/HAN23080480/UI/IngameHUD/WBP_ModeDescription.TextBlock_DescLine1` _aswbp_mode_description) "Classic Mode but with power-up pick ups.")
  (`TextBlock.SetText` (`/Game/HAN23080480/UI/IngameHUD/WBP_ModeDescription.TextBlock_DescLine2` _aswbp_mode_description) "Good Luck and Have fun!")
  (set `self.Level Name` "FiestaLevel"))

(fn `UserConstructionScript`
  (`parent.UserConstructionScript`))