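; Player-linked landmine that explodes after a timer, or when a Player-tagged actor or projectile overlaps it once PlayerREF leaving opens the gate.
; A looping timeline blinks the material and plays a timer sound; its rate derives from the countdown, which currently decrements by zero.
; The one-shot explosion damages sphere-trace hits, spawns effects, then, if PlayerREF is valid, updates its mine count message and destroys the mine.
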(event `self.ReceiveBeginPlay`
  (bind _landmine (`self.Landmine`))
  (set `self.CurrentTimeBeforeExplosion` (`self.TimeBeforeExplosion`))
  (`TimelineComponent.SetPlayRate` (`self.Timeline`) (/ 1.0 (/ (`self.CurrentTimeBeforeExplosion`) 5.0)))
  (`|ExecutionSequence`
    (:`then_0`
      ;[1 1 1] Timer death condition
      (`KismetSystemLibrary.Delay` (`self.TimeBeforeExplosion`))
      (`/Engine/EditorBlueprintResources/StandardMacros.DoOnce` false
        (:`Completed`
          (`self.ExplosionDamge`))))
    (:`then_1`
      ;[1 1 1] Timer decreasing
      (`KismetSystemLibrary.Delay` 1.0 :!label _label)
      (set `self.CurrentTimeBeforeExplosion` (- (`self.CurrentTimeBeforeExplosion`) 0.0))
      (goto _label))
    (:`then_2`
      ;[1 1 1] Ticking Material
      (bind (_direction _color_changer) (`Timeline|Timeline` :!via `PlayFromStart` :!label _label_2)
        (:`Update`
          (switch `int` (`KismetMathLibrary.FTrunc` _color_changer)
            (:`0`
              (`PrimitiveComponent.SetMaterial` _landmine 1 "/Game/LevelPrototyping/Materials/MI_Solid_Blue.MI_Solid_Blue"))
            (:`1`
              (`PrimitiveComponent.SetMaterial` _landmine 1 "/Game/NguyenQuangHuy/Assets/Mesh/Object/Mine/Red.Red")))
          (`TimelineComponent.SetPlayRate` (`self.Timeline`) (/ 1.0 (/ (`self.CurrentTimeBeforeExplosion`) 5.0))))
        (:`Finished`
          (`/Engine/EditorBlueprintResources/StandardMacros.IsValid` self
            (:`Is Valid`
              (`GameplayStatics.SpawnSoundAtLocation` "/Game/NguyenQuangHuy/Assets/SFX/SFX/S_MineTimer.S_MineTimer" (`self.K2_GetActorLocation`) (struct) 1.0 1.0 0.0 null null)
              (goto _label_2 :!via `PlayFromStart`))))))))

(event `self.Capsule.OnComponentBeginOverlap`
  (params (OverlappedComponent :type "PrimitiveComponent Object Reference") (OtherActor :type "Actor Object Reference") (OtherComp :type "PrimitiveComponent Object Reference") (OtherBodyIndex :type Integer) (bFromSweep :type Boolean) (SweepResult :type "HitResult Structure (by ref)"))
  (`/Engine/EditorBlueprintResources/StandardMacros.Gate` true :!label _label_3
    (:`Exit`
      (if (not (`self.ActorHasTag` OtherActor "Player"))
        (cast `/Game/Phong/Blueprints/BP_Projectile_Master` OtherActor))
      (`self.ExplosionDamge`))))

(event `self.Capsule.OnComponentEndOverlap`
  (params (OverlappedComponent :type "PrimitiveComponent Object Reference") (OtherActor :type "Actor Object Reference") (OtherComp :type "PrimitiveComponent Object Reference") (OtherBodyIndex :type Integer))
  (if (== OtherActor (`self.Player REF`))
    (goto _label_3 :!via `Open`)))

(fn `ExplosionDamge`
  (bind _returnvalue (`self.K2_GetActorLocation`))
  (bind _returnvalue_2 (`self.K2_GetActorLocation`))
  (bind _player_ref (`self.Player REF`))
  (`/Engine/EditorBlueprintResources/StandardMacros.DoOnce` false
    (:`Completed`
      (bind _outhits (`KismetSystemLibrary.SphereTraceMulti` _returnvalue _returnvalue (`self.Radius`) "TraceTypeQuery5"))
      (for _array_element _outhits
        (`GameplayStatics.ApplyDamage` (`.HitActor` (`GameplayStatics.BreakHitResult` _array_element)) (`self.Damage`)))
      (`GameplayStatics.SpawnEmitterAtLocation` "/Game/Realistic_Starter_VFX_Pack_Vol2/Particles/Explosion/P_Explosion_Big_A.P_Explosion_Big_A" _returnvalue_2)
      (`GameplayStatics.SpawnSoundAtLocation` "/Game/NguyenQuangHuy/Assets/SFX/SFX/S_TankDeath.S_TankDeath" _returnvalue_2 (struct) 1.0 1.0 0.0 null null)
      (`/Engine/EditorBlueprintResources/StandardMacros.IsValid` _player_ref
        (:`Is Valid`
          (message `/Game/NguyenQuangHuy/Blueprints/Mine/BPI_MineCount.UpdateMineCount` _player_ref)
          (`self.K2_DestroyActor`))))))

(fn `UserConstructionScript`)