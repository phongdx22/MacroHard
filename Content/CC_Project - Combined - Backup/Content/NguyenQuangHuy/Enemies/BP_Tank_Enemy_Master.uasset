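; Master enemy tank Blueprint that hunts and shoots the player, with a tintable material and a health bar.
; A 0.2-second timer loop fires when a muzzle trace, optionally with one ricochet, hits a "Tank"-tagged actor, limited by fire rate and bullet count.
; The cannon tracks the player with a precision-based random offset, and PawnSensing starts an AI chase.
; At zero health it explodes, notifies the game mode and is destroyed.
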(event `self.ReceiveBeginPlay`
  (set `self.Life` (`self.Life_Max`))
  (bind _returnvalue (`self.UpdateTankColor` (`self.Tank Color`)))
  (`PrimitiveComponent.SetMaterial` (`self.CannonMesh`) 0 _returnvalue)
  (`PrimitiveComponent.SetMaterial` (`self.Mesh`) 0 _returnvalue)
  (`self.Event Main`)
  (set `self.BulletCountMax` 5)
  (bind _aswbp_health_bar (cast `/Game/HAN23080480/UI/IngameHUD/WBP_HealthBar` (`WidgetComponent.GetUserWidgetObject` (`self.Widget_HealthBar`))))
  (set `/Game/HAN23080480/UI/IngameHUD/WBP_HealthBar.HealthBarColour` (struct :`R` 0.25 :`G` 0.05 :`A` 1.0) _aswbp_health_bar)
  (`ProgressBar.SetPercent` (`/Game/HAN23080480/UI/IngameHUD/WBP_HealthBar.HealthBar` _aswbp_health_bar) (`self.Life_Max`)))

(event `Event Main`
  (`|ExecutionSequence`
    (:`then_0`
      (`KismetSystemLibrary.K2_SetTimerDelegate` (delegate `Event Main`) 0.2)
      (bind _should_shoot_ (`self.Scope Trace Test`))
      (if _should_shoot_
        (bind _canweshoot_ (`self.CanShoot?`))
        (if _canweshoot_
          (`/Engine/EditorBlueprintResources/StandardMacros.DoOnce` false :!label _label
            (:`Completed`
              (`self.Shoot`)
              (`KismetSystemLibrary.Delay` (`self.FireRate`))
              (goto _label :!via `Reset`))))))
    (:`then_1`
      (`KismetSystemLibrary.Delay` (`self.PrecisionRate`))
      (bind _target_location (`self.PrecisionScope`))
      (set `self.Target Location` _target_location))))

(event `self.ReceiveTick`
  (params (DeltaSeconds :type "Float (single-precision)"))
  (bind (_returnvalue_roll _returnvalue_pitch _returnvalue_yaw) (`KismetMathLibrary.BreakRotator` (`SceneComponent.K2_GetComponentRotation` (`self.CannonMesh`))))
  (bind (_returnvalue_roll_2 _returnvalue_pitch_2 _returnvalue_yaw_2) (`KismetMathLibrary.BreakRotator` (`KismetMathLibrary.FindLookAtRotation` (`self.K2_GetActorLocation`) (`self.Target Location`))))
  (`SceneComponent.K2_SetWorldRotation` (`self.CannonMesh`) (`KismetMathLibrary.RInterpTo` (`KismetMathLibrary.MakeRotator` 0.0 0.0 _returnvalue_yaw) (`KismetMathLibrary.MakeRotator` 0.0 0.0 (- _returnvalue_yaw_2 90.0)) (`GameplayStatics.GetWorldDeltaSeconds`) (`self.Precision Speed`)) false false))

(event `self.ReceiveAnyDamage`
  (params (Damage :type "Float (single-precision)") (DamageType :type "DamageType Object Reference") (InstigatedBy :type "Controller Object Reference") (DamageCauser :type "Actor Object Reference"))
  (bind _output_get (set `self.Life` (- (`self.Life`) Damage)))
  (bind _aswbp_health_bar (cast `/Game/HAN23080480/UI/IngameHUD/WBP_HealthBar` (`WidgetComponent.GetUserWidgetObject` (`self.Widget_HealthBar`))))
  (bind _returnvalue (/ _output_get (`self.Life_Max`)))
  (`ProgressBar.SetPercent` (`/Game/HAN23080480/UI/IngameHUD/WBP_HealthBar.HealthBar` _aswbp_health_bar) _returnvalue)
  (if (<= _returnvalue 0.0)
    (`GameplayStatics.SpawnEmitterAtLocation` "/Game/StarterContent/Particles/P_Explosion.P_Explosion" (`SceneComponent.K2_GetComponentLocation` (`self.Mesh`)))
    (message `/Game/NguyenQuangHuy/InterFaces/BP_Tank_SurvivalGameMode.EnemyKilled` (`GameplayStatics.GetGameMode`))
    (`self.K2_DestroyActor`)))

(event `Shoot`
  (bind (_returnvalue_location _returnvalue_rotation) (`KismetMathLibrary.BreakTransform` (`SceneComponent.K2_GetComponentToWorld` (`self.Muzzle`))))
  ;[1 1 1] Shoot
  (bind _canweshoot_ (`self.CanShoot?`))
  (if _canweshoot_
    (`/Engine/EditorBlueprintResources/StandardMacros.IncrementInt` (`self.BulletCount`)
      (:`  `
        (`|SpawnActorFromClass` (`self.ProjectileToShoot`) (`KismetMathLibrary.MakeTransform` _returnvalue_location _returnvalue_rotation) "Undefined" "MultiplyWithRoot" null self 10.0 null)
        (`GameplayStatics.SpawnSoundAtLocation` "/Game/NguyenQuangHuy/Assets/SFX/SFX/S_Fireshot_Classic.S_Fireshot_Classic" _returnvalue_location (struct) 1.0 1.0 0.0 null null)))))

(event `/Game/NguyenQuangHuy/InterFaces/BPI_BulletCount.UpdateBulletCount`
  ;[1 1 1] Shoot
  (`/Engine/EditorBlueprintResources/StandardMacros.DecrementInt` (`self.BulletCount`)))

(event `self.PawnSensing.OnSeePawn`
  (params (Pawn :type "Pawn Object Reference"))
  ;[1 1 1] If see player,  chase player
  (if (`self.ActorHasTag` Pawn "Player")
    (if (`KismetMathLibrary.RandomBoolWithWeight` 1.0)
      (if (not (`self.ChasingPlayer?`))
        (set `self.PlayerRef` Pawn)
        (`self.ChasePlayer`)))))

(event `ChasePlayer`
  ;[1 1 1] Attack player event
  (if (and (not (`self.IsDead?`)) (not (`self.ChasingPlayer?`)) (not (`self.IsChasingKeep`)) (not (`self.IsAttacking?`)))
    (set `self.ChasingPlayer?` true)
    (`|AIMoveTo` self (0.0 0.0 0.0) (`self.PlayerRef`))))

(fn `CanMine?`
  (returns (ReturnValue :type Boolean))
  (return (< (`self.MineCount`) (`self.MineCountMax`))))

(fn `CanShoot?`
  (returns (`CanWeShoot?` :type Boolean))
  (return (< (`self.BulletCount`) (`self.BulletCountMax`))))

(fn `PrecisionScope`
  (returns (`Target Location` :type "Vector Structure"))
  (locals (TempTargetLoc :type "Vector Structure"))
  (switch `/Game/NguyenQuangHuy/Enemies/ENUM_Precision` (`self.Precision`)
    (:`NewEnumerator0`
      (set `self.PrecisionOffset` 400.0))
    (:`NewEnumerator1`
      (set `self.PrecisionOffset` 200.0))
    (:`NewEnumerator2`
      (set `self.PrecisionOffset` 100.0))
    (:`NewEnumerator3`
      (set `self.PrecisionOffset` 0.0)))
  (bind _output_get (set `local.TempTargetLoc` (+ (`self.K2_GetActorLocation` (`GameplayStatics.GetPlayerCharacter` 0)) (* (`KismetMathLibrary.GetRightVector` (`KismetMathLibrary.FindLookAtRotation` (`self.K2_GetActorLocation` (`GameplayStatics.GetPlayerCharacter` 0)) (`self.K2_GetActorLocation`))) (`KismetMathLibrary.RandomFloatInRange` (* (`self.PrecisionOffset`) -1.0) (`self.PrecisionOffset`))))))
  (return _output_get))

(fn `Scope Trace Test`
  (returns (`Should Shoot?` :type Boolean))
  (bind _muzzle (`self.Muzzle`))
  (bind _returnvalue (`SceneComponent.K2_GetComponentLocation` _muzzle))
  (bind _returnvalue_2 (+ _returnvalue (* (`SceneComponent.GetForwardVector` _muzzle) (`self.TraceDistance`))))
  (bind (_outhit _returnvalue_3) (`KismetSystemLibrary.LineTraceSingle` :`Start` _returnvalue :`End` _returnvalue_2 :`TraceChannel` "TraceTypeQuery1" :`DrawTime` 0.2))
  (if _returnvalue_3
    (bind (_bblockinghit _binitialoverlap _time _distance _location _impactpoint _normal _impactnormal _physmat _hitactor) (`GameplayStatics.BreakHitResult` _outhit))
    (if (`self.ActorHasTag` _hitactor "Tank")
      (return true)
      (elif (`self.Bounce?`)
        (bind _returnvalue_4 (`KismetMathLibrary.FindLookAtRotation` (+ _impactpoint _normal) (+ _impactpoint (`KismetMathLibrary.MirrorVectorByNormal` (* _returnvalue_2 (`SceneComponent.K2_GetComponentLocation` (`self.Muzzle`))) _normal))))
        (bind (_outhit_2 _returnvalue_5) (`KismetSystemLibrary.LineTraceSingle` :`Start` (+ _impactpoint (* (`KismetMathLibrary.GetForwardVector` _returnvalue_4) 50.0)) :`End` (* (`KismetMathLibrary.GetForwardVector` _returnvalue_4) (`self.TraceDistance`)) :`TraceChannel` "TraceTypeQuery1" :`DrawTime` 0.2))
        (if _returnvalue_5
          (if (`self.ActorHasTag` (`.HitActor` (`GameplayStatics.BreakHitResult` _outhit_2)) "Tank")
            (return true)
            (else
              (return false)))
          (else
            (return false)))
        (else
          (return false))))
    (elif (not (`self.Bounce?`))
      (return false))))

(fn `UpdateTankColor`
  (params (Value :type "LinearColor Structure"))
  (returns (ReturnValue :type "MaterialInstanceDynamic Object Reference"))
  (bind _returnvalue (`KismetMaterialLibrary.CreateDynamicMaterialInstance` "/Game/NguyenQuangHuy/Enemies/M_Tank_Enemy_Color.M_Tank_Enemy_Color" "None"))
  (`MaterialInstanceDynamic.SetVectorParameterValue` _returnvalue "Color" Value)
  (return _returnvalue))

(fn `UserConstructionScript`
  (bind _returnvalue (`self.UpdateTankColor` (`self.Tank Color`)))
  (`PrimitiveComponent.SetMaterial` (`self.CannonMesh`) 0 _returnvalue)
  (`PrimitiveComponent.SetMaterial` (`self.Mesh`) 0 _returnvalue))