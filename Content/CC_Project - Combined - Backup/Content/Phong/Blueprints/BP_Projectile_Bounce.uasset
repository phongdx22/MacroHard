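; BP_Projectile_Bounce is a projectile that bounces a limited number of times before it is destroyed.
; Each bounce event from its ProjectileMovement component increments BounceCount and calls DestroyBullet when the count equals BounceCountMax.
; BeginPlay, overlap and Tick are disabled stubs, and the construction script only calls the parent, so the bounce limit is the only logic in this Blueprint.
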(event `self.ProjectileMovement.OnProjectileBounce`
  (params (ImpactResult :type "HitResult Structure (by ref)") (ImpactVelocity :type "Vector Structure (by ref)"))
  (bind _result (`/Engine/EditorBlueprintResources/StandardMacros.IncrementInt` (`self.BounceCount`))
    (:`  `
      (if (== _result (`self.BounceCountMax`))
        (`self.Destroy Bullet`)))))

(fn `UserConstructionScript`
  (`parent.UserConstructionScript`))