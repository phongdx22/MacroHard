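; Master tank projectile that damages actors tagged "Tank" on hit, then destroys itself with an impact sound.
; On BeginPlay it copies the instigator tank's sniper, multishot and big-tank flags; sniper shots delay destruction, and non-multishot bullets also self-destruct when velocity reaches zero.
; On destruction it tells the instigator to update its bullet count message.
; Line-trace ricochet logic with a bounce limit exists, but its event graph chain never runs.
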(event `self.ReceiveBeginPlay`
  (bind _asbp_tank_player (cast `/Game/Phong/Blueprints/BP_TankPlayer` (`self.Instigator REF`)))
  (set `self.Sniping?` (`/Game/Phong/Blueprints/BP_TankPlayer.SniperShot?` _asbp_tank_player))
  (set `self.Multishooting?` (`/Game/Phong/Blueprints/BP_TankPlayer.Multishot?` _asbp_tank_player))
  (set `self.BigBullet?` (`/Game/Phong/Blueprints/BP_TankPlayer.BigTank?` _asbp_tank_player)))

(event `self.ReceiveTick`
  (params (DeltaSeconds :type "Float (single-precision)"))
  (if (`self.Multishooting?`)
    _
    (elif (== (`self.GetVelocity`) (0.0 0.0 0.0))
      (`/Engine/EditorBlueprintResources/StandardMacros.DoOnce` false
        (:`Completed`
          (`self.Destroy Bullet`))))))

(event `self.ReceiveDestroyed`
  (bind _instigator_ref (`self.Instigator REF`))
  (`/Engine/EditorBlueprintResources/StandardMacros.IsValid` _instigator_ref
    (:`Is Valid`
      (message `/Game/NguyenQuangHuy/InterFaces/BPI_BulletCount.UpdateBulletCount` _instigator_ref))))

(event `Destroy Bullet`
  (`GameplayStatics.SpawnSoundAtLocation` "/Game/NguyenQuangHuy/Assets/SFX/SFX/S_BulletHitWall.S_BulletHitWall" (`SceneComponent.K2_GetComponentLocation` (`self.ForwardArrow`)) (struct) 1.0 1.0 0.0 null null)
  (if (`self.Sniping?`)
    (`KismetSystemLibrary.Delay` 0.4))
  (`self.K2_DestroyActor`))

(event `self.ReceiveHit`
  (params (MyComp :type "PrimitiveComponent Object Reference") (Other :type "Actor Object Reference") (OtherComp :type "PrimitiveComponent Object Reference") (bSelfMoved :type Boolean) (HitLocation :type "Vector Structure") (HitNormal :type "Vector Structure") (NormalImpulse :type "Vector Structure") (Hit :type "HitResult Structure (by ref)"))
  (if (`self.ActorHasTag` Other "Tank")
    (`GameplayStatics.ApplyDamage` Other (`self.Base Damage`))
    (`self.Destroy Bullet`)))

(fn `Bounce`
  (params (Hit :type "HitResult Structure") (Origin :type "Vector Structure") (Forward :type "Vector Structure"))
  (bind (_bblockinghit _binitialoverlap _time _distance _location _impactpoint _normal _impactnormal) (`GameplayStatics.BreakHitResult` Hit))
  (`self.K2_SetActorRotation` (`KismetMathLibrary.FindLookAtRotation` (+ _impactpoint _normal) (+ (`KismetMathLibrary.MirrorVectorByNormal` (- Forward Origin) _normal) _impactpoint)))
  (set `MovementComponent.Velocity` (`KismetMathLibrary.MirrorVectorByNormal` (`MovementComponent.Velocity` (`self.ProjectileMovement`)) _impactnormal) (`self.ProjectileMovement`))
  (`GameplayStatics.SpawnSoundAtLocation` "/Game/NguyenQuangHuy/Assets/SFX/SFX/S_Ricochet.S_Ricochet" (`SceneComponent.K2_GetComponentLocation` (`self.ForwardArrow`)) (struct) 1.0 1.0 0.0 null null))

(fn `CheckIfCanBounce`
  (returns (`CanBounce?` :type Boolean))
  (if (< (`self.BounceCount`) (`self.BounceCountMax`))
    (return true)
    (else
      (return false))))

(fn `TestTraceDetectionDamageable`
  (returns (OutHit :type "HitResult Structure") (ReturnValue :type Boolean) (Origin :type "Vector Structure") (Forward :type "Vector Structure"))
  (bind _forwardarrow (`self.ForwardArrow`))
  (bind _returnvalue (`SceneComponent.K2_GetComponentLocation` _forwardarrow))
  (`/Engine/EditorBlueprintResources/StandardMacros.IsValid` _forwardarrow
    (:`Is Valid`
      (bind (_outhit _returnvalue_2) (`KismetSystemLibrary.LineTraceSingle` _returnvalue (+ _returnvalue (* (`SceneComponent.GetForwardVector` _forwardarrow) (`self.TraceDistance`))) "TraceTypeQuery5"))
      (return _outhit _returnvalue_2 (0.0 0.0 0.0) (0.0 0.0 0.0)))))

(fn `TestTraceDetectionEnvironment`
  (returns (OutHit :type "HitResult Structure") (ReturnValue :type Boolean) (Origin :type "Vector Structure") (Forward :type "Vector Structure"))
  (bind _forwardarrow (`self.ForwardArrow`))
  (bind _returnvalue (`SceneComponent.K2_GetComponentLocation` _forwardarrow))
  (bind _returnvalue_2 (+ _returnvalue (* (`SceneComponent.GetForwardVector` _forwardarrow) (`self.TraceDistance`))))
  (bind (_outhit _returnvalue_3) (`KismetSystemLibrary.LineTraceSingle` _returnvalue _returnvalue_2 "TraceTypeQuery4"))
  (return _outhit _returnvalue_3 _returnvalue _returnvalue_2))

(fn `UserConstructionScript`)