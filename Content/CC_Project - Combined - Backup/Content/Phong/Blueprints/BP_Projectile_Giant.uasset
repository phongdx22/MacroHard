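; BP_Projectile_Giant is a giant projectile, a child Blueprint that damages actors tagged "Tank" and explodes on contact.
; Its DamageSphere overlap applies BaseDamage to tanks and spawns P_Explosion at the sweep location.
; Any other overlap spawns the same explosion and calls DestroyBullet, while tank hits leave the projectile alive in this graph.
; BeginPlay and construction defer to the parent class.
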(event `self.ReceiveBeginPlay`
  (`parent.ReceiveBeginPlay`))

(event `self.DamageSphere.OnComponentBeginOverlap`
  (params (OverlappedComponent :type "PrimitiveComponent Object Reference") (OtherActor :type "Actor Object Reference") (OtherComp :type "PrimitiveComponent Object Reference") (OtherBodyIndex :type Integer) (bFromSweep :type Boolean) (SweepResult :type "HitResult Structure (by ref)"))
  (bind (_bblockinghit _binitialoverlap _time _distance _location) (`GameplayStatics.BreakHitResult` SweepResult))
  (if (`self.ActorHasTag` OtherActor "Tank")
    (`GameplayStatics.ApplyDamage` OtherActor (`self.Base Damage`))
    (`GameplayStatics.SpawnEmitterAtLocation` "/Game/StarterContent/Particles/P_Explosion.P_Explosion" _location)
    (else
      (`GameplayStatics.SpawnEmitterAtLocation` "/Game/StarterContent/Particles/P_Explosion.P_Explosion" _location)
      (`self.Destroy Bullet`))))

(fn `UserConstructionScript`
  (`parent.UserConstructionScript`))