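; BP_Projectile_Explode is an explosive projectile that deals area damage on impact.
; Its Hit event applies radial damage with falloff around the hit location, ignoring the projectile itself, then spawns an explosion particle effect and a tank-death sound there.
; The graph does not destroy the actor, and its BeginPlay, overlap and Tick events are disabled placeholders.
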(event `self.ReceiveHit`
  (params (MyComp :type "PrimitiveComponent Object Reference") (Other :type "Actor Object Reference") (OtherComp :type "PrimitiveComponent Object Reference") (bSelfMoved :type Boolean) (HitLocation :type "Vector Structure") (HitNormal :type "Vector Structure") (NormalImpulse :type "Vector Structure") (Hit :type "HitResult Structure (by ref)"))
  (`GameplayStatics.ApplyRadialDamageWithFalloff` 25.0 5.0 HitLocation 50.0 300.0 4.0 null (`|MakeArray` self :!type "Actor Object Reference") null null)
  (`GameplayStatics.SpawnEmitterAtLocation` "/Game/StarterContent/Particles/P_Explosion.P_Explosion" HitLocation)
  (`GameplayStatics.SpawnSoundAtLocation` "/Game/NguyenQuangHuy/Assets/SFX/SFX/S_TankDeath.S_TankDeath" HitLocation (struct) 1.0 1.0 0.0 null null))

(fn `UserConstructionScript`
  (`parent.UserConstructionScript`))