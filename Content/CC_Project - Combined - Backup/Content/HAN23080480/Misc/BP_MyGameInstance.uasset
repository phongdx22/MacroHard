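; Game instance that runs shuffled background music which persists across level transitions.
; Init fills a list of five BGM tracks and shuffles it.
; PlayMusic and PlayNewTrack share a NewTrack-gated path that spawns a 2D sound and schedules PlayNewTrack by timer.
; The index increments before the timer reads the duration, so the delay uses the following track's length, and the index never wraps.
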(event `Play New Track`
  (bind _output (`|GetArrayItem` (`self.MusicList`) (`self.MusicIndex`)))
  (set `self.NewTrack?` true)
  (if (`self.NewTrack?`) :!label _label
    (`GameplayStatics.SpawnSound2D` _output 0.5 1.0 0.0 null true)
    (`/Engine/EditorBlueprintResources/StandardMacros.IncrementInt` (`self.MusicIndex`)
      (:`  `
        (`KismetSystemLibrary.K2_SetTimerDelegate` (delegate `Play New Track`) (`SoundBase.Duration` _output))
        (set `self.NewTrack?` false)))))

(event `self.ReceiveInit`
  (bind _output_get (set `self.MusicList` (`|MakeArray` "/Game/HAN23080480/Sounds/Music/BGM_Beat_Them_Up_1_by_Jan_Chmelar.BGM_Beat_Them_Up_1_by_Jan_Chmelar" "/Game/HAN23080480/Sounds/Music/BGM_Beat_Them_Up_3_by_Jan_Chmelar.BGM_Beat_Them_Up_3_by_Jan_Chmelar" "/Game/HAN23080480/Sounds/Music/BGM_Concrete_Jungle_10_by_Jan_Chmelar.BGM_Concrete_Jungle_10_by_Jan_Chmelar" "/Game/HAN23080480/Sounds/Music/BGM_Hit_The_Floor_14_by_Jan_Chmelar.BGM_Hit_The_Floor_14_by_Jan_Chmelar" "/Game/HAN23080480/Sounds/Music/BGM_The_Race_Around_the_World_-_Waterflame.BGM_The_Race_Around_the_World_-_Waterflame" :!type "SoundBase Object Reference")))
  (`KismetArrayLibrary.Array_Shuffle` _output_get))

(event `PlayMusic`
  (goto _label))