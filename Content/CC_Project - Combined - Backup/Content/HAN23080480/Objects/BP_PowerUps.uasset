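; BP_PowerUps is a pickup actor that grants power-up components to the player's tank.
; A BP_TankPlayer overlapping its sphere gets AddPowerUpsComponents and destroys the pickup; damage instigated by that tank's controller also grants them, without destroying it.
; After a pickup is collected, it counts remaining BP_PowerUps actors and calls Reset on GM_PowerUps when none are left.
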(event `self.ReceiveAnyDamage`
  (params (Damage :type "Float (single-precision)") (DamageType :type "DamageType Object Reference") (InstigatedBy :type "Controller Object Reference") (DamageCauser :type "Actor Object Reference"))
  (bind _asplayer_controller (cast `PlayerController` InstigatedBy))
  (bind _asbp_tank_player (cast `/Game/Phong/Blueprints/BP_TankPlayer` (`Controller.K2_GetPawn` _asplayer_controller)))
  (`AddComponent|NODE_AddPowerUpsComponents-1` :`self` _asbp_tank_player))

(event `self.Sphere.OnComponentBeginOverlap`
  (params (OverlappedComponent :type "PrimitiveComponent Object Reference") (OtherActor :type "Actor Object Reference") (OtherComp :type "PrimitiveComponent Object Reference") (OtherBodyIndex :type Integer) (bFromSweep :type Boolean) (SweepResult :type "HitResult Structure (by ref)"))
  (bind _asbp_tank_player (cast `/Game/Phong/Blueprints/BP_TankPlayer` OtherActor))
  (`AddComponent|NODE_AddPowerUpsComponents-0` :`self` _asbp_tank_player)
  (`self.K2_DestroyActor`)
  (bind _outactors (`GameplayStatics.GetAllActorsOfClass` "BP_PowerUps_C"))
  (if (== (`KismetArrayLibrary.Array_Length` _outactors) 0)
    (bind _asgm_power_ups (cast `/Game/HAN23080480/Gamemodes/GM_PowerUps` (`GameplayStatics.GetGameMode`)))
    (`/Game/HAN23080480/Gamemodes/GM_PowerUps.Reset` _asgm_power_ups)))

(fn `UserConstructionScript`)